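; Base enemy Blueprint for MagicExploration that takes flat and burn damage and destroys itself when health runs out.
; Interface calls feed a shared TakeDamage function, directly for flat hits or through a looping timer for burning.
; Burn re-application resets duration and elapsed time rather than stacking timers.
; It also returns its Body location as the lightning target, and prints debug damage and health values.
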(event `/Game/MagicExploration/Blueprints/Interfaces/I_Character.ITakeDamage`
  (params (Amount :type Integer))
  ;[1 1 1] Debug
  (`KismetSystemLibrary.PrintString` (`KismetStringLibrary.Concat_StrStr` "Flat Damage: " (`KismetStringLibrary.Conv_IntToString` Amount)) true true (struct :`G` 0.66 :`B` 1.0 :`A` 1.0) (`self.DebugStringDuration`))
  (`self.TakeDamage` Amount))

(event `/Game/MagicExploration/Blueprints/Interfaces/I_Character.IStartBurning`
  (params (BurnDamage :type Integer) (Tick :type "Float (single-precision)") (BurnDuration :type "Float (single-precision)"))
  (set `self.BurningDuration` BurnDuration)
  (set `self.BurningElapsed` 0.0)
  (if (not (`self.IsBurnning`))
    (set `self.IsBurnning` true)
    (bind _returnvalue (`KismetSystemLibrary.K2_SetTimerDelegate` (delegate `TakeDamageOverTime`) Tick true))
    (set `self.BurningTimerHandle` _returnvalue)))

(event `TakeDamageOverTime`
  ;[1 1 1] Debug
  (`KismetSystemLibrary.PrintString` (`KismetStringLibrary.Concat_StrStr` "DOT: " (`KismetStringLibrary.Conv_IntToString` (stale `/Game/MagicExploration/Blueprints/Interfaces/I_Character.IStartBurning` BurnDamage))) true true (struct :`G` 0.66 :`B` 1.0 :`A` 1.0) (`self.DebugStringDuration`))
  (`self.TakeDamage` (stale `/Game/MagicExploration/Blueprints/Interfaces/I_Character.IStartBurning` BurnDamage))
  (bind _output_get (set `self.BurningElapsed` (+ (stale `/Game/MagicExploration/Blueprints/Interfaces/I_Character.IStartBurning` Tick) (`self.BurningElapsed`))))
  (if (>= _output_get (`self.BurningDuration`))
    (`KismetSystemLibrary.K2_ClearAndInvalidateTimerHandle` (`self.BurningTimerHandle`))
    (set `self.IsBurnning` false)))

(fn `IGetLightningTargetLocation`
  (returns (Location :type "Vector Structure"))
  (return (`SceneComponent.K2_GetComponentLocation` (`self.Body`))))

(fn `TakeDamage`
  (params (Value :type Integer))
  (bind _output_get (set `self.Health` (- (`self.Health`) Value)))
  ;[1 1 1] Debug
  (`KismetSystemLibrary.PrintString` (`KismetStringLibrary.Concat_StrStr` "Remaining health: " (`KismetStringLibrary.Conv_IntToString` (`self.Health`))) true true (struct :`G` 0.66 :`B` 1.0 :`A` 1.0) (`self.DebugStringDuration`))
  (if (not (> _output_get 0))
    (`self.K2_DestroyActor`))
  (return))

(fn `UserConstructionScript`)