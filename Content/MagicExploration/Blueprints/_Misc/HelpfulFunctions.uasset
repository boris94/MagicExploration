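; HelpfulFunctions is a set of small utility functions for negating numbers and querying status effect tiers.
; InvertFloat and InvertInt flip the sign of their input.
; HasHigherForm and HasLowerForm use the effect's enum name as the row key into StatusEffectsDataTable.
; Each returns the linked form and whether it differs from a sentinel enum value, with no handling for missing rows.
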(fn `HasHigherForm`
  (params (StatusEffect :type "/Game/MagicExploration/Blueprints/StatusEffects/StatusEffect Enum" :default "NewEnumerator4"))
  (returns (Has :type Boolean) (HigherForm :type "/Game/MagicExploration/Blueprints/StatusEffects/StatusEffect Enum"))
  (bind _returnvalue (`|GetDataTableRow` "/Game/MagicExploration/Blueprints/StatusEffects/StatusEffectsDataTable.StatusEffectsDataTable" (`KismetStringLibrary.Conv_StringToName` (`|GetEnumeratorNameAsString` StatusEffect)))
    (:`then`
      (bind (_lowerform _higherform) (break `/Game/MagicExploration/Blueprints/StatusEffects/StatusEffectsDTStruct` _returnvalue))
      (return (not (`|EnumEquality` _higherform "NewEnumerator4")) _higherform))))

(fn `HasLowerForm`
  (params (StatusEffect :type "/Game/MagicExploration/Blueprints/StatusEffects/StatusEffect Enum" :default "NewEnumerator4"))
  (returns (Has :type Boolean) (LowerForm :type "/Game/MagicExploration/Blueprints/StatusEffects/StatusEffect Enum"))
  (bind _returnvalue (`|GetDataTableRow` "/Game/MagicExploration/Blueprints/StatusEffects/StatusEffectsDataTable.StatusEffectsDataTable" (`KismetStringLibrary.Conv_StringToName` (`|GetEnumeratorNameAsString` StatusEffect)))
    (:`then`
      (bind ((`LowerForm_6_08E0E5D64123613F98C2C4B9072524D4` _lowerform)) (break `/Game/MagicExploration/Blueprints/StatusEffects/StatusEffectsDTStruct` _returnvalue))
      (return (not (`|EnumEquality` _lowerform "NewEnumerator4")) _lowerform))))

(fn `InvertFloat`
  (params (value :type "Float (double-precision)"))
  (returns (result :type "Float (double-precision)"))
  (return (* value -1.0)))

(fn `InvertInt`
  (params (Value :type Integer))
  (returns (Result :type Integer))
  (return (* Value -1)))