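; Status effect manager component that applies Burning, Aflame, Chilled and Frozen to its owner.
; A shared BaseApply macro rejects immune, already active or outranked effects, removes lower forms, then expires the effect after a delay.
; Burning and Aflame loop damage ticks through an interface message while active.
; Chilled reduces walk speed; Frozen disables movement and sets the IsStunned blackboard key, then turns into Chilled on expiry.
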(event `ApplyBurning`
  (params (Duration :type "Float (double-precision)") (Damage :type Integer) (Tick :type "Float (double-precision)"))
  ;[1 1 1] Burning
  (bind _appliedeffect (`self.BaseApply` "NewEnumerator0" (+ Duration (`KismetMathLibrary.FClamp` Tick Tick 0.1)))
    (:`then`
      (`KismetSystemLibrary.Delay` Tick :!label _label)
      (if (`KismetArrayLibrary.Array_Contains` (`self.ActiveStatusEffects`) _appliedeffect)
        (message `/Game/MagicExploration/Blueprints/Interfaces/I_Damagable.ITakeDamage` (`self.GetOwner`) Damage)
        (goto _label)))))

(event `ApplyAflame`
  (params (Duration :type "Float (double-precision)") (Damage :type Integer) (Tick :type "Float (double-precision)"))
  ;[1 1 1] Aflame
  (bind _appliedeffect (`self.BaseApply` "NewEnumerator1" (+ Duration (`KismetMathLibrary.FClamp` Tick Tick 0.1)))
    (:`then`
      (`KismetSystemLibrary.Delay` Tick :!label _label_2)
      (if (`KismetArrayLibrary.Array_Contains` (`self.ActiveStatusEffects`) _appliedeffect)
        (message `/Game/MagicExploration/Blueprints/Interfaces/I_Damagable.ITakeDamage` (`self.GetOwner`) Damage)
        (goto _label_2)))))

(event `ApplyChilled`
  (params (Durtion :type "Float (double-precision)") (SlowPercentage :type "Float (double-precision)"))
  (bind _returnvalue (`Actor.GetComponentByClass` (`self.GetOwner`) "/Script/Engine.CharacterMovementComponent"))
  (bind _maxwalkspeed (`CharacterMovementComponent.MaxWalkSpeed` _returnvalue))
  (bind _returnvalue_2 (* _maxwalkspeed (/ SlowPercentage 100.0)))
  ;[1 1 1] Chilled
  (`self.BaseApply` "NewEnumerator2" Durtion
    (:`OnRemove`
      (`self.RemoveChilledSlow`))
    (:`then`
      (`/Engine/EditorBlueprintResources/StandardMacros.IsValid` _returnvalue
        (:`Is Valid`
          (set `self.AppliedChilledSlow` _returnvalue_2)
          (set `CharacterMovementComponent.MaxWalkSpeed` (- _maxwalkspeed _returnvalue_2) _returnvalue)
          ;;[1 1 1] debug
          (`KismetSystemLibrary.PrintString` "Slow applied" true true (struct :`G` 0.66 :`B` 1.0 :`A` 1.0) 30.0))))))

(event `ApplyFrozen`
  (params (StunDuration :type "Float (double-precision)") (SlowDuration :type "Float (double-precision)") (SlowPercentage :type "Float (double-precision)"))
  (bind _returnvalue (`self.GetOwner`))
  (bind _returnvalue_2 (`self.GetOwner`))
  ;[1 1 1] Frozen
  (`self.BaseApply` "NewEnumerator3" StunDuration
    (:`OnRemoveLowerForm`
      (`self.RemoveChilledSlow`))
    (:`OnRemove`
      (`CharacterMovementComponent.SetMovementMode` (`Actor.GetComponentByClass` _returnvalue "/Script/Engine.CharacterMovementComponent") "MOVE_Walking" 0)
      (`BlackboardComponent.SetValueAsBool` (`AIBlueprintHelperLibrary.GetBlackboard` _returnvalue) (`KismetStringLibrary.Conv_StringToName` "IsStunned") false)
      (`self.ApplyChilled` SlowDuration SlowPercentage))
    (:`then`
      (`CharacterMovementComponent.DisableMovement` (`Actor.GetComponentByClass` _returnvalue_2 "/Script/Engine.CharacterMovementComponent"))
      (`BlackboardComponent.SetValueAsBool` (`AIBlueprintHelperLibrary.GetBlackboard` _returnvalue_2) (`KismetStringLibrary.Conv_StringToName` "IsStunned") true))))

(fn `BaseRemoveStatusEffect`
  (params (StatusEffect :type "/Game/MagicExploration/Blueprints/StatusEffects/StatusEffect Enum" :default "NewEnumerator4"))
  (`KismetArrayLibrary.Array_RemoveItem` (`self.ActiveStatusEffects`) StatusEffect)
  (return))

(fn `RemoveChilledSlow`
  (bind _returnvalue (`Actor.GetComponentByClass` (`self.GetOwner`) "/Script/Engine.CharacterMovementComponent"))
  ;[1 1 1] Debug
  (`KismetSystemLibrary.PrintString` "SlowRemoved" true true (struct :`G` 0.66 :`B` 1.0 :`A` 1.0) 30.0)
  (`self.BaseRemoveStatusEffect` "NewEnumerator2")
  (`/Engine/EditorBlueprintResources/StandardMacros.IsValid` _returnvalue
    (:`Is Valid`
      (set `CharacterMovementComponent.MaxWalkSpeed` (+ (`CharacterMovementComponent.MaxWalkSpeed` _returnvalue) (`self.AppliedChilledSlow`)) _returnvalue)
      (return))))