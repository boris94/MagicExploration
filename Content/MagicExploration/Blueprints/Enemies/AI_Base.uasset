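; Base enemy Blueprint with health that can take damage and be targeted by lightning.
; BeginPlay seeds two Blackboard points, Target1 at a fixed Y offset from the spawn location and Target2 at the spawn location itself.
; Interface calls feed damage into TakeDamage, which lowers Health, prints debug text and destroys the actor at zero or below.
; Another interface function returns the actor's location as the lightning target.
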(event `self.ReceiveBeginPlay`
  (bind _returnvalue (`AIBlueprintHelperLibrary.GetBlackboard` self))
  (bind _returnvalue_2 (`self.K2_GetActorLocation` self))
  (`BlackboardComponent.SetValueAsVector` _returnvalue (`self.Target1`) (`KismetMathLibrary.MakeVector` (.x _returnvalue_2) (+ (.y _returnvalue_2) 1200.0) (.z _returnvalue_2)))
  (`BlackboardComponent.SetValueAsVector` _returnvalue (`self.Target2`) _returnvalue_2))

(event `/Game/MagicExploration/Blueprints/Interfaces/I_Damagable.ITakeDamage`
  (params (Amount :type Integer))
  ;[1 1 1] Debug
  (`KismetSystemLibrary.PrintString` (`KismetStringLibrary.Concat_StrStr` "Damage: " (`KismetStringLibrary.Conv_IntToString` Amount)) true true (struct :`G` 0.66 :`B` 1.0 :`A` 1.0) 30.0)
  (`self.TakeDamage` Amount))

(fn `IGetLightningTargetLocation`
  (returns (Location :type "Vector Structure"))
  (bind (_returnvalue_x _returnvalue_y _returnvalue_z) (`KismetMathLibrary.BreakVector` (`self.K2_GetActorLocation`)))
  (return (`KismetMathLibrary.MakeVector` _returnvalue_x _returnvalue_y _returnvalue_z)))

(fn `TakeDamage`
  (params (Amount :type Integer))
  (bind _output_get (set `self.Health` (- (`self.Health`) Amount)))
  ;[1 1 1] Debug
  (`KismetSystemLibrary.PrintString` (`KismetStringLibrary.Concat_StrStr` "Remaining health: " (`KismetStringLibrary.Conv_IntToString` (`self.Health`))) true true (struct :`G` 0.66 :`B` 1.0 :`A` 1.0) 30.0)
  (if (not (> _output_get 0))
    (`self.K2_DestroyActor`)))

(fn `UserConstructionScript`)