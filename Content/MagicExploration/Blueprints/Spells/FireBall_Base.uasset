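; FireBall_Base is the fireball spell actor that damages and ignites what its Area component overlaps.
; Overlaps with the player or a LightningBeam are ignored.
; Any other actor receives damage and burn-over-time interface messages, then the fireball destroys itself.
; A separate PendDestroy event destroys it after a short delay.
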(event `PendDestroy`
  (`KismetSystemLibrary.Delay` 2.0)
  (`self.K2_DestroyActor`))

(event `self.Area.OnComponentBeginOverlap`
  (params (OverlappedComponent :type "PrimitiveComponent Object Reference") (OtherActor :type "Actor Object Reference") (OtherComp :type "PrimitiveComponent Object Reference") (OtherBodyIndex :type Integer) (bFromSweep :type Boolean) (SweepResult :type "HitResult Structure (by ref)"))
  (if (not (or (`.bSuccess` (cast `/Game/MagicExploration/Blueprints/Characters/ME_Player` OtherActor :!pure true)) (`.bSuccess` (cast `/Game/MagicExploration/Blueprints/Spells/LightningBeam` OtherActor :!pure true))))
    (message `/Game/MagicExploration/Blueprints/Interfaces/I_Character.ITakeDamage` OtherActor (`self.Damage`))
    (message `/Game/MagicExploration/Blueprints/Interfaces/I_Character.IStartBurning` OtherActor (`self.DamageOverTime`) 1.0 5.0)
    (`self.K2_DestroyActor`)))

(fn `UserConstructionScript`)