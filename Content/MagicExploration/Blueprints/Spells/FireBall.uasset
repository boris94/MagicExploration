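; Fireball spell actor that damages and ignites whatever its Area overlaps, ignoring the player and LightningBeam actors.
; Charging up calls the parent logic and rescales the mesh; charged hits use separate damage and burn-over-time values.
; Damage and burning go through interface messages, then the fireball destroys itself if the target is still valid.
; A PendDestroy event also destroys it after a short delay.
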(event `self.ChargeUp`
  (`parent.ChargeUp`)
  (`SceneComponent.SetWorldScale3D` (`self.StaticMesh`) (0.2 0.2 0.2)))

(event `PendDestroy`
  (`KismetSystemLibrary.Delay` 2.0)
  (`self.K2_DestroyActor`))

(event `self.Area.OnComponentBeginOverlap`
  (params (OverlappedComponent :type "PrimitiveComponent Object Reference") (OtherActor :type "Actor Object Reference") (OtherComp :type "PrimitiveComponent Object Reference") (OtherBodyIndex :type Integer) (bFromSweep :type Boolean) (SweepResult :type "HitResult Structure (by ref)"))
  (if (not (or (`.bSuccess` (cast `/Game/MagicExploration/Blueprints/Characters/ME_Player` OtherActor :!pure true)) (`.bSuccess` (cast `/Game/MagicExploration/Blueprints/Spells/LightningBeam` OtherActor :!pure true))))
    (if (`self.IsCharged`)
      (`/Engine/EditorBlueprintResources/StandardMacros.IsValid` OtherActor
        (:`Is Valid`
          (message `/Game/MagicExploration/Blueprints/Interfaces/I_Enemy.ITakeDamage` OtherActor (`self.ChargedDamage`))
          (`/Engine/EditorBlueprintResources/StandardMacros.IsValid` OtherActor
            (:`Is Valid`
              (message `/Game/MagicExploration/Blueprints/Interfaces/I_Enemy.IStartBurning` OtherActor (`self.ChargedBurnDOT`) (`self.ChargedBurnTick`) (`self.ChargedBurnDuration`))))))
      (else
        (`/Engine/EditorBlueprintResources/StandardMacros.IsValid` OtherActor
          (:`Is Valid`
            (message `/Game/MagicExploration/Blueprints/Interfaces/I_Enemy.ITakeDamage` OtherActor (`self.Damage`))
            (`/Engine/EditorBlueprintResources/StandardMacros.IsValid` OtherActor
              (:`Is Valid`
                (message `/Game/MagicExploration/Blueprints/Interfaces/I_Enemy.IStartBurning` OtherActor (`self.BurnDOT`) (`self.BurnTick`) (`self.BurnDuration`))))))))
    (`self.K2_DestroyActor`)))

(fn `UserConstructionScript`)