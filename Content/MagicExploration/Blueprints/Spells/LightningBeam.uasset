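; Lightning beam spell that locks onto an I_Enemy entering its Range, damaging it immediately and then on a looping timer.
; Overlap also begins the inherited charge; once charged, damage switches to the charged value and the particle template changes.
; Tick and construction update the beam endpoints, targeting the enemy's interface-provided location or a default Target component.
; An enemy leaving Range resets the charge, timer and target.
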(event `self.StopCharge`
  (`parent.StopCharge`)
  (set `self.IsCharged` false)
  (`ParticleSystemComponent.SetTemplate` (`self.ParticleSystem`) "/Game/MagicExploration/Particles/LightningBeam.LightningBeam"))

(event `self.ReceiveTick`
  (params (DeltaSeconds :type "Float (single-precision)"))
  (`self.UpdateBeamPosistion`))

(event `self.ChargeUp`
  (`parent.ChargeUp`)
  (`ParticleSystemComponent.SetTemplate` (`self.ParticleSystem`) "/Game/MagicExploration/Particles/LightningBeam_Charged.LightningBeam_Charged"))

(event `self.Range.OnComponentBeginOverlap`
  (params (OverlappedComponent :type "PrimitiveComponent Object Reference") (OtherActor :type "Actor Object Reference") (OtherComp :type "PrimitiveComponent Object Reference") (OtherBodyIndex :type Integer) (bFromSweep :type Boolean) (SweepResult :type "HitResult Structure (by ref)"))
  (if (`KismetSystemLibrary.DoesImplementInterface` OtherActor "/Game/MagicExploration/Blueprints/Interfaces/I_Enemy.I_Enemy_C")
    (set `self.Enemy` OtherActor)
    (`self.DealDamage`)
    (`self.BeginCharge`)
    (`KismetSystemLibrary.K2_SetTimer` null "DealDamage" (`self.DamageTick`) true)))

(event `self.Range.OnComponentEndOverlap`
  (params (OverlappedComponent :type "PrimitiveComponent Object Reference") (OtherActor :type "Actor Object Reference") (OtherComp :type "PrimitiveComponent Object Reference") (OtherBodyIndex :type Integer))
  (if (`KismetSystemLibrary.DoesImplementInterface` OtherActor "/Game/MagicExploration/Blueprints/Interfaces/I_Enemy.I_Enemy_C")
    (`self.StopCharge`)
    (`KismetSystemLibrary.K2_ClearTimer` null "DealDamage")
    (set `self.Enemy` null)))

(fn `DealDamage`
  (bind _enemy (`self.Enemy`))
  (if (`self.IsCharged`)
    (`/Engine/EditorBlueprintResources/StandardMacros.IsValid` _enemy
      (:`Is Valid`
        (message `/Game/MagicExploration/Blueprints/Interfaces/I_Enemy.ITakeDamage` _enemy (`self.ChargedDamage`))))
    (else
      (`/Engine/EditorBlueprintResources/StandardMacros.IsValid` _enemy
        (:`Is Valid`
          (message `/Game/MagicExploration/Blueprints/Interfaces/I_Enemy.ITakeDamage` _enemy (`self.Damage`))))))
  (return))

(fn `UpdateBeamPosistion`
  (bind _particlesystem (`self.ParticleSystem`))
  (`ParticleSystemComponent.SetBeamSourcePoint` (`self.ParticleSystem`) 0 (`SceneComponent.K2_GetComponentLocation` (`self.Scene`)) 0)
  (`/Engine/EditorBlueprintResources/StandardMacros.IsValid` (`self.Enemy`)
    (:`Is Valid`
      (bind _location (message `/Game/MagicExploration/Blueprints/Interfaces/I_Enemy.IGetLightningTargetLocation` (`self.Enemy`)))
      (`ParticleSystemComponent.SetBeamTargetPoint` _particlesystem 0 _location 0))
    (:`Is Not Valid`
      (`ParticleSystemComponent.SetBeamTargetPoint` _particlesystem 0 (`SceneComponent.K2_GetComponentLocation` (`self.Target`)) 0))))

(fn `UserConstructionScript`
  (`self.UpdateBeamPosistion`))